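; Game mode for a bullet-hell game that spawns enemy waves and handles start and end screens and level progression.
; After BeginPlay loads the save, SpawnEnemies reads numbered rows from the DataTable picked by TestLevel, not the saved level.
; Each row drives delayed, repeated batches of enemies with velocity, destination and projectile rotation, then recursively triggers the next.
; GameOver shows the result and, on non-final wins, saves progress and opens the next level.
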(event Custom|Spawn%20Enemies
  (bind _spawnsequencecounter (Variables|Default|GetSpawnSequenceCounter))
  (bind _returnvalue (Utilities|String|ToString(Integer) _spawnsequencecounter))
  (bind _returnvalue_2 (Utilities|String|StringToName _returnvalue))
  (switch int (Variables|Default|GetTestLevel)
    (:0
      (bind _returnvalue_3 (Utilities|GetDataTableRow "/Game/Blueprints/DT_EnemySpawns_Level01.DT_EnemySpawns_Level01" _returnvalue_2)
        (:then
          (Variables|Default|SetEnemySpawnStruct _returnvalue_3)
          (Development|PrintString _returnvalue :!label _label)
          (Utilities|FlowControl|Delay (.spawncountdelay (Variables|Default|GetEnemySpawnStruct)) :!label _label_2)
          (for _index (range 0 (- (.enemycount (Variables|Default|GetEnemySpawnStruct)) 1))
            (bind _returnvalue_4 (Game|SpawnActorfromClass (Utilities|Array|Get(acopy) (Variables|Default|GetEnemyClasses) (Utilities|Array|Get(acopy) (.enemytype (Variables|Default|GetEnemySpawnStruct)) _index)) (Math|Transform|MakeTransform (Utilities|Array|Get(acopy) (.spawnlocation (Variables|Default|GetEnemySpawnStruct)) _index) (Utilities|Array|Get(acopy) (.spawnrotation (Variables|Default|GetEnemySpawnStruct)) _index) "1.000000,1.000000,1.000000") "AlwaysSpawn" "MultiplyWithRoot" 0 0))
            (Class|EnemyShip|SetVelocity _returnvalue_4 (.x (Utilities|Array|Get(acopy) (.xyvelocity (Variables|Default|GetEnemySpawnStruct)) _index)) (.y (Utilities|Array|Get(acopy) (.xyvelocity (Variables|Default|GetEnemySpawnStruct)) _index)))
            (Class|EnemyShip|SetDestination _returnvalue_4 (Utilities|Array|Get(acopy) (.destination (Variables|Default|GetEnemySpawnStruct)) _index))
            (Class|EnemyShip|SetProjectileRotationOffset _returnvalue_4 (Utilities|Array|Get(acopy) (.projectilerotation (Variables|Default|GetEnemySpawnStruct)) _index)))
          (bind _result (Math|Integer|IncrementInt (Variables|Default|Getindex))
            (:%20%20
              (if (< _result (.spawncount (Variables|Default|GetEnemySpawnStruct)))
                (goto _label_2)
                (else
                  (Variables|Default|Setindex 0)
                  (Math|Integer|IncrementInt (Variables|Default|GetSpawnSequenceCounter)
                    (:%20%20
                      (Utilities|FlowControl|Delay (.delaybeforenextsequence (Variables|Default|GetEnemySpawnStruct)))
                      (CallFunction|SpawnEnemies))))))))
        (:RowNotFound
          (Development|PrintString "Finished Spawning" :!label _label_3))))
    (:1
      (bind _returnvalue_5 (Utilities|GetDataTableRow "/Game/Blueprints/DT_EnemySpawns_Level02.DT_EnemySpawns_Level02" _returnvalue_2)
        (:then
          (Variables|Default|SetEnemySpawnStruct _returnvalue_5)
          (goto _label))
        (:RowNotFound
          (goto _label_3))))
    (:2
      (bind _returnvalue_6 (Utilities|GetDataTableRow "/Game/Blueprints/DT_EnemySpawns_Level03.DT_EnemySpawns_Level03" _returnvalue_2)
        (:then
          (Variables|Default|SetEnemySpawnStruct _returnvalue_6)
          (goto _label))
        (:RowNotFound
          (goto _label_3))))))

(event EventBeginPlay
  (bind _returnvalue (SaveGame|LoadGamefromSlot "1"))
  (bind _asbp_save_reference (Utilities|Casting|CastToBP_SaveReference _returnvalue))
  (Variables|Default|SetSaveReference _asbp_save_reference)
  (Utilities|FlowControl|Delay 3.0)
  (CallFunction|SpawnEnemies))

(event EventTick
  (params (DeltaSeconds :type Float%20%28single-precision%29)))

(event EventStartGame
  (bind _returnvalue (UserInterface|CreateWidget "/Game/Widgets/WBP_StartGameWidget.WBP_StartGameWidget_C"))
  (UserInterface|Viewport|AddtoViewport _returnvalue 0))

(event EventGameOver
  (params (bWonGame :type Boolean))
  (bind _savereference (Variables|Default|GetSaveReference))
  (bind _returnvalue (UserInterface|CreateWidget "/Game/Widgets/WBP_EndGameWidget.WBP_EndGameWidget_C"))
  (UserInterface|Viewport|AddtoViewport _returnvalue 0)
  (Rendering|Components|TextRender|SetText (Variables|/Game/Widgets/WBP_EndGameWidget.WBP_EndGameWidget_C|GetDisplayText _returnvalue) (Utilities|Text|ToText(String) (select bWonGame "YOU WON!" "YOU LOSE!")))
  (if bWonGame
    (if (<= (Variables|/Game/Blueprints/BP_SaveReference.BP_SaveReference_C|GetCurrentLevel _savereference) 1)
      (Utilities|Array|SetArrayElem (Variables|/Game/Blueprints/BP_SaveReference.BP_SaveReference_C|GetLevelProgress _savereference) (Variables|/Game/Blueprints/BP_SaveReference.BP_SaveReference_C|GetCurrentLevel _savereference) true)
      (bind _result (Math|Integer|IncrementInt (Variables|/Game/Blueprints/BP_SaveReference.BP_SaveReference_C|GetCurrentLevel _savereference))
        (:%20%20
          (bind _output_get (Variables|/Game/Blueprints/BP_SaveReference.BP_SaveReference_C|SetCurrentLevel _savereference _result))
          (SaveGame|SaveGametoSlot _savereference "1")
          (Utilities|FlowControl|Delay 4.0)
          (switch int _output_get
            (:1
              (Game|OpenLevel(byObjectReference) "/Game/Maps/Level02.Level02"))
            (:2
              (Game|OpenLevel(byObjectReference) "/Game/Maps/Level03.Level03")))))
      (else
        (Development|PrintString "Finished Game ROLL CREDITS")
        (Utilities|FlowControl|Delay 5.0)))))

(fn ConstructionScript)